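; Health component that tracks damage and death for its owning actor.
; Damage events clear the owner's AI blackboard "Stunned?" flag, then subtract clamped health unless the damage causer shares the damaged actor's class, preventing same-class damage.
; A death check fires the Death dispatcher when health runs out, and Reset restores health to maximum.
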(event Custom|Reset
  (Variables|Default|SetHealth (Variables|Default|GetMaxHealth)))

(event Custom|Damaged
  (params (DamagedActor :type Actor%20Object%20Reference) (Damage :type Float%20%28single-precision%29) (DamageType :type E_DamageTypes%20Enum :default "NewEnumerator0") (InstigatedBy :type Controller%20Object%20Reference) (DamageCauser :type Actor%20Object%20Reference))
  (bind _returnvalue (Components|GetOwner))
  (bind _returnvalue_2 (AI|GetAIController _returnvalue))
  (bind _returnvalue_3 (AI|GetBlackboard _returnvalue_2))
  (Utilities|IsValid DamagedActor
    (:Is%20Valid
      (Utilities|IsValid _returnvalue_3
        (:Is%20Valid
          (AI|Components|Blackboard|SetValueasBool _returnvalue_3 (Utilities|Name|MakeLiteralName "Stunned?") false))
        (:Is%20Not%20Valid
          _))
      (if (!= (Utilities|GetClass DamagedActor) (Utilities|GetClass DamageCauser))
        (Variables|Default|SetHealth (Math|Float|Clamp(Float) (- (Variables|Default|GetHealth) Damage) 0.0 (Variables|Default|GetMaxHealth)))
        (CallFunction|DeathCheck)))))

(event Custom|DeathCheck
  (if (<= (Variables|Default|GetHealth) 0.0)
    (Default|CallDeath)))