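; Camera trigger actor that switches the level's BP_Camera between two preset locations as the player passes through it.
; Leaving Box alternates the camera position through a FlipFlop and rotates Box to face the matching side.
; Entering Box1 moves the camera to the opposite position a tick later, then advances the FlipFlop with a Flipped flag so its state stays in sync without moving the camera again.
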(event OnComponentEndOverlap(Box)
  (params (OverlappedComponent :type Primitive%20Component%20Object%20Reference) (OtherActor :type Actor%20Object%20Reference) (OtherComp :type Primitive%20Component%20Object%20Reference) (OtherBodyIndex :type Integer))
  (bind _cam (Variables|Default|GetCam))
  (if (== OtherActor (Game|GetPlayerCharacter 0))
    (Utilities|FlowControl|FlipFlop
      (:A
        (if (Variables|Default|GetFlipped)
          (Variables|Default|SetFlipped false)
          (Variables|Default|SetLocation 0.0)
          (else
            (Transformation|SetActorLocation _cam (Variables|Default|GetLocation1) false false)
            (Transformation|SetWorldRotation (Variables|Default|GetBox) "0.000000,-180.000000,0.000000" false false)
            (Variables|Default|SetLocation 0.0))))
      (:B
        (if (Variables|Default|GetFlipped)
          (Variables|Default|SetFlipped false)
          (Variables|Default|SetLocation 1.0)
          (else
            (Transformation|SetActorLocation _cam (Variables|Default|GetLocation2) false false)
            (Transformation|SetWorldRotation (Variables|Default|GetBox) "0, 0, 0" false false)
            (Variables|Default|SetLocation 1.0)))))))

(event OnComponentBeginOverlap(Box1)
  (params (OverlappedComponent :type Primitive%20Component%20Object%20Reference) (OtherActor :type Actor%20Object%20Reference) (OtherComp :type Primitive%20Component%20Object%20Reference) (OtherBodyIndex :type Integer) (bFromSweep :type Boolean) (SweepResult :type Hit%20Result%20Structure%20%28by%20ref%29))
  (if (== OtherActor (Game|GetPlayerCharacter 0))
    (if (== (Variables|Default|GetLocation) 0.0)
      (Utilities|FlowControl|DelayUntilNextTick)
      (Transformation|SetActorLocation (Variables|Default|GetCam) (Variables|Default|GetLocation2) false false)
      (Transformation|SetWorldRotation (Variables|Default|GetBox) "0, 0, 0" false false)
      (else
        (Utilities|FlowControl|DelayUntilNextTick)
        (Transformation|SetActorLocation (Variables|Default|GetCam) (Variables|Default|GetLocation1) false false)
        (Transformation|SetWorldRotation (Variables|Default|GetBox) "0.000000,-180.000000,0.000000" false false)))
    (Variables|Default|SetFlipped true)
    (CallFunction|Flip)))

(event Custom|Flip
  (bind _cam (Variables|Default|GetCam))
  (Utilities|FlowControl|FlipFlop
    (:A
      (if (Variables|Default|GetFlipped)
        (Variables|Default|SetFlipped false)
        (Variables|Default|SetLocation 0.0)
        (else
          (Transformation|SetActorLocation _cam (Variables|Default|GetLocation1) false false)
          (Transformation|SetWorldRotation (Variables|Default|GetBox) "0.000000,-180.000000,0.000000" false false)
          (Variables|Default|SetLocation 0.0))))
    (:B
      (if (Variables|Default|GetFlipped)
        (Variables|Default|SetFlipped false)
        (Variables|Default|SetLocation 1.0)
        (else
          (Transformation|SetActorLocation _cam (Variables|Default|GetLocation2) false false)
          (Transformation|SetWorldRotation (Variables|Default|GetBox) "0, 0, 0" false false)
          (Variables|Default|SetLocation 1.0))))))

(event EventBeginPlay
  (bind _returnvalue (Actor|GetActorOfClass "/Game/Player/BP_Camera.BP_Camera_C"))
  (Variables|Default|SetCam _returnvalue))

(fn ConstructionScript)