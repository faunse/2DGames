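; Base 2D enemy AI character that handles damage reactions and exposes its EnemyPath.
; Damage is forwarded to the health component; type 0 also stops movement, sets Blackboard stun and state keys, and runs a death check.
; While the Blackboard Dead key is unset, each damage branch plays its own timeline to flash the sprite through a dynamic material.
; The health component's Death event stops both timelines and clears the flash.
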(event Death(BPC_Health)
  (CallFunction|Stop))

(event Custom|Stop
  (bind _material (Variables|Default|GetMaterial))
  (bind _material_2 (Variables|Default|GetMaterial))
  (Utilities|FlowControl|Sequence
    (:then_0
      (bind (_direction _invincibletime _newtrack_1) (Timeline|Timeline_0 Stop)
        (:Update
          (Rendering|Material|SetScalarParameterValue _material_2 "Flash" _invincibletime :!class /Script/Engine.MaterialInstanceDynamic)
          (Rendering|Material|SetVectorParameterValue _material_2 "FlashColour" _newtrack_1 :!class /Script/Engine.MaterialInstanceDynamic))
        (:Finished
          (Rendering|Material|SetScalarParameterValue (Variables|Default|GetMaterial) "Flash" 0.0 :!class /Script/Engine.MaterialInstanceDynamic))))
    (:then_1
      (bind (_direction_2 _invincibletime_2 _newtrack_1_2) (Timeline|Timeline Stop)
        (:Update
          (Rendering|Material|SetScalarParameterValue _material "Flash" _invincibletime_2 :!class /Script/Engine.MaterialInstanceDynamic)
          (Rendering|Material|SetVectorParameterValue _material "FlashColour" _newtrack_1_2 :!class /Script/Engine.MaterialInstanceDynamic))))
    (:then_2
      (Rendering|Material|SetScalarParameterValue (Variables|Default|GetMaterial) "Flash" 0.0 :!class /Script/Engine.MaterialInstanceDynamic))))

(event Collision|EventActorBeginOverlap
  (params (OtherActor :type Actor%20Object%20Reference)))

(event EventTick
  (params (DeltaSeconds :type Float%20%28single-precision%29)))

(event EventBeginPlay
  (bind _returnvalue (Rendering|Material|CreateDynamicMaterialInstance (Variables|Default|GetSprite) 0 0 "None" :!class /Script/Engine.PrimitiveComponent))
  (Variables|Default|SetMaterial _returnvalue))

(event EventApply/TakeDamage
  (params (Damaged%20Actor :type Actor%20Object%20Reference) (Damage%20amount :type Float%20%28double-precision%29) (Damage%20type :type E_DamageTypes%20Enum :default "NewEnumerator0") (Damage%20Causer :type Actor%20Object%20Reference))
  (bind _returnvalue (Pawn|GetController))
  (bind _material (Variables|Default|GetMaterial))
  (bind _material_2 (Variables|Default|GetMaterial))
  (bind _returnvalue_2 (AI|GetBlackboard _returnvalue))
  (Default|Damaged (Variables|Default|GetBPC_Health) Damaged%20Actor Damage%20amount Damage%20type 0 Damage%20Causer)
  (if (== Damage%20type 0)
    (Components|Movement|StopMovementImmediately (Variables|Character|GetCharacterMovement))
    (AI|Components|Blackboard|SetValueasBool _returnvalue_2 (Utilities|Name|MakeLiteralName "Stunned?") true)
    (AI|Components|Blackboard|SetValueasEnum _returnvalue_2 (Utilities|Name|MakeLiteralName "States") (Utilities|Enum|LiteralenumE_States "NewEnumerator2"))
    (Utilities|FlowControl|Sequence
      (:then_0
        (if (not (ScalableFloat|GetValueasBool (AI|GetBlackboard (Pawn|GetController)) (Utilities|Name|MakeLiteralName "Dead")))
          (bind (_direction _invincibletime _newtrack_1) (Timeline|Timeline_0 PlayFromStart)
            (:Update
              (Rendering|Material|SetScalarParameterValue _material_2 "Flash" _invincibletime :!class /Script/Engine.MaterialInstanceDynamic)
              (Rendering|Material|SetVectorParameterValue _material_2 "FlashColour" _newtrack_1 :!class /Script/Engine.MaterialInstanceDynamic))
            (:Finished
              (Rendering|Material|SetScalarParameterValue (Variables|Default|GetMaterial) "Flash" 0.0 :!class /Script/Engine.MaterialInstanceDynamic)))))
      (:then_1
        (Default|DeathCheck (Variables|Default|GetBPC_Health))))
    (elif (not (ScalableFloat|GetValueasBool (AI|GetBlackboard (Pawn|GetController)) (Utilities|Name|MakeLiteralName "Dead")))
      (bind (_direction_2 _invincibletime_2 _newtrack_1_2) (Timeline|Timeline PlayFromStart)
        (:Update
          (Rendering|Material|SetScalarParameterValue _material "Flash" _invincibletime_2 :!class /Script/Engine.MaterialInstanceDynamic)
          (Rendering|Material|SetVectorParameterValue _material "FlashColour" _newtrack_1_2 :!class /Script/Engine.MaterialInstanceDynamic))))))

(fn ConstructionScript)

(fn GetPath
  (return (Variables|Default|GetEnemyPath)))