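; BP_Necromancer is a 2D enemy character with 500 health and a shield that toggles its invincibility.
; BeginPlay registers its enemy type in the AI Blackboard, while StartFight and Stun write the Blackboard's States value.
; StateChange jumps the animation state machine to the node named after the state, raising the shield for attack states and dropping it when stunned.
; The shield also lowers sprite opacity as a visual cue.
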(event Custom|Stun
  (AI|Components|Blackboard|SetValueasEnum (AI|GetBlackboard (Pawn|GetController)) (Utilities|Name|MakeLiteralName "States") (Utilities|Enum|LiteralenumE_States "NewEnumerator2")))

(event Custom|ShieldUp
  (bind _papersprite (Variables|Default|GetPaperSprite))
  (bind _spritecolor (Variables|/Script/Paper2D.PaperSpriteComponent|GetSpriteColor _papersprite))
  (Sprite|SetSpriteColor _papersprite (Utilities|Struct|MakeLinearColor (.r _spritecolor) (.g _spritecolor) (.b _spritecolor) 0.3))
  (Variables|Default|SetInvincible? true))

(event Custom|ShieldDown
  (bind _papersprite (Variables|Default|GetPaperSprite))
  (bind _spritecolor (Variables|/Script/Paper2D.PaperSpriteComponent|GetSpriteColor _papersprite))
  (Sprite|SetSpriteColor _papersprite (Utilities|Struct|MakeLinearColor (.r _spritecolor) (.g _spritecolor) (.b _spritecolor) 0.0))
  (Variables|Default|SetInvincible? false))

(event Custom|StartFight
  (AI|Components|Blackboard|SetValueasEnum (AI|GetBlackboard (Pawn|GetController)) (Utilities|Name|MakeLiteralName "States") (Utilities|Enum|LiteralenumE_States "NewEnumerator1")))

(event EventBeginPlay
  (bind _bpc_health (Variables|Default|GetBPC_Health))
  (|CallParentFunction)
  (AI|Components|Blackboard|SetValueasEnum (AI|GetBlackboard (Pawn|GetController)) (Utilities|Name|MakeLiteralName "EnemyType") (Utilities|Enum|LiteralenumE_EnemyType "NewEnumerator2"))
  (bind _output_get (Variables|/Game/Components/BPC_Health.BPC_Health_C|SetMaxHealth _bpc_health 5e+02))
  (Variables|/Game/Components/BPC_Health.BPC_Health_C|SetHealth _bpc_health _output_get))

(event Collision|EventActorBeginOverlap
  (params (OtherActor :type Actor%20Object%20Reference))
  (|CallParentFunction OtherActor) ; This node is disabled and will not be called.\nDrag off pins to build functionality.
)

(event EventStateChange
  (params (States :type E_AnimStates%20Enum :default "NewEnumerator0"))
  (bind _returnvalue (Utilities|String|EnumtoString States))
  (bind _returnvalue_2 (Utilities|String|StringToName _returnvalue))
  (Development|PrintString (Utilities|String|ToString(Name) _returnvalue_2))
  (Class|PaperZDAnimInstance|JumptoNode (Variables|/Script/PaperZD.PaperZDAnimationComponent|GetAnimInstance (Variables|Default|GetAnimationComponent)) _returnvalue_2 "None")
  (switch Utilities|FlowControl|Switch|SwitchonE_AnimStates States
    (:NewEnumerator2
      (CallFunction|ShieldUp))
    (:NewEnumerator3
      (CallFunction|ShieldDown))
    (:NewEnumerator4
      (CallFunction|ShieldUp))))

(fn ConstructionScript
  (|CallParentFunction))