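; BP_NecroFire is a Necromancer enemy fire projectile, shown as a flipbook sprite, that damages the player on contact.
; On spawn it attaches a looping-or-one-shot fire sound and a timeline animates the sprite's dynamic material flash, activating projectile movement when finished.
; Box overlap with the player sends a damage message, calls an empty SFX event and destroys the actor, which also cleans up the sound.
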(event OnComponentBeginOverlap(Box)
  (params (OverlappedComponent :type Primitive%20Component%20Object%20Reference) (OtherActor :type Actor%20Object%20Reference) (OtherComp :type Primitive%20Component%20Object%20Reference) (OtherBodyIndex :type Integer) (bFromSweep :type Boolean) (SweepResult :type Hit%20Result%20Structure%20%28by%20ref%29))
  (bind _returnvalue (Game|GetPlayerCharacter 0))
  (if (== OtherActor _returnvalue)
    (Class|BPIDamage|Apply/TakeDamage(Message) _returnvalue OtherActor 1.0 "NewEnumerator1")
    (CallFunction|SFX)
    (Actor|DestroyActor)))

(event Custom|SFX)

(event EventBeginPlay
  (bind _returnvalue (Rendering|Material|CreateDynamicMaterialInstance (Variables|Default|GetPaperFlipbook) 0 0 "None" :!class /Script/Engine.PrimitiveComponent))
  (bind _returnvalue_2 (Audio|SpawnSoundAttached "/Game/Sound/Sounds/MSS_Fire2.MSS_Fire2" (Variables|Default|GetPaperFlipbook) "None" "0, 0, 0" "0, 0, 0" "KeepRelativeOffset" false 1.0 1.0 0.0 0 "/Game/Sound/Sounds/SC_Fire.SC_Fire"))
  (Variables|Default|SetFireSound _returnvalue_2)
  (Variables|Default|SetMaterial _returnvalue)
  (bind (_direction _invincibletime _newtrack_1) (Timeline|Timeline PlayFromStart)
    (:Update
      (Rendering|Material|SetScalarParameterValue (Variables|Default|GetMaterial) "Flash" _invincibletime :!class /Script/Engine.MaterialInstanceDynamic)
      (Rendering|Material|SetVectorParameterValue (Variables|Default|GetMaterial) "FlashColour" _newtrack_1 :!class /Script/Engine.MaterialInstanceDynamic))
    (:Finished
      (Components|Activation|Activate (Variables|Default|GetProjectileMovement) false))))

(event EventDestroyed
  (bind _firesound (Variables|Default|GetFireSound))
  (Utilities|IsValid _firesound
    (:Is%20Valid
      (Components|DestroyComponent _firesound))))

(fn ConstructionScript)