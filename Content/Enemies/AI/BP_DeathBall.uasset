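; BP_DeathBall is an enemy homing projectile, a ghost ball that chases the player character and damages it on contact.
; On spawn it homes on the first child of the player's capsule, plays a ghost-ball sound and starts a lifetime timer.
; A box overlap with the player applies damage and destroys it immediately.
; Otherwise, the timer swaps its flipbook to an explosion, then removes it shortly after.
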(event OnComponentBeginOverlap(Box)
  (params (OverlappedComponent :type Primitive%20Component%20Object%20Reference) (OtherActor :type Actor%20Object%20Reference) (OtherComp :type Primitive%20Component%20Object%20Reference) (OtherBodyIndex :type Integer) (bFromSweep :type Boolean) (SweepResult :type Hit%20Result%20Structure%20%28by%20ref%29))
  (if (== OtherActor (Game|GetPlayerCharacter 0))
    (Class|BPIDamage|Apply/TakeDamage(Message) OtherActor OtherActor 1.0 "NewEnumerator1" self)
    (Actor|DestroyActor)))

(event Custom|Destroy
  (Sprite|SetFlipbook (Variables|Default|GetFB_Ball) "/Game/Art/Ball/FB_BallExplodes.FB_BallExplodes")
  (Utilities|Time|SetTimerbyEvent (delegate Custom|Explode) 0.5))

(event Custom|Explode
  (Actor|DestroyActor))

(event EventBeginPlay
  (Variables|/Script/Engine.ProjectileMovementComponent|SetHomingTargetComponent (Variables|Default|GetProjectileMovement) (Components|GetChildComponent (Variables|/Script/Engine.Character|GetCapsuleComponent (Game|GetPlayerCharacter 0)) 0))
  (Audio|SpawnSoundatLocation "/Game/Sound/Sounds/MSS_GhostBall.MSS_GhostBall" (Transformation|GetActorLocation) "0, 0, 0" 3.0 1.0 0.0 0 "/Game/Sound/Sounds/SC_GhostBall.SC_GhostBall")
  (Utilities|Time|SetTimerbyEvent (delegate Custom|Destroy) 3.5))

(fn ConstructionScript)