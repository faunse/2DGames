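; BP_SkullSpawner is an enemy spawner that spawns a BPAI_Skull at its Arrow component and respawns it after it is destroyed.
; On BeginPlay it plays a ghost spawn sound, waits briefly, then spawns the skull and binds to its OnDestroyed event.
; The death handler is set up to re-enter the same spawn sequence through a short timer, forming a respawn loop.
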(event Custom|Respawn
  (bind _arrow (Variables|Default|GetArrow))
  (bind _returnvalue (Transformation|GetWorldLocation _arrow))
  (Audio|SpawnSoundatLocation "/Game/Sound/Sounds/MSS_GhostSpawn.MSS_GhostSpawn" _returnvalue "0, 0, 0" 1.0 1.0 0.0 0 "/Game/Sound/Sounds/SC_GhostSpawn.SC_GhostSpawn")
  (Utilities|FlowControl|Delay 0.2)
  (bind _returnvalue_2 (Game|SpawnActorfromClass "/Game/Enemies/AI/BPAI_Skull.BPAI_Skull_C" (Math|Transform|MakeTransform _returnvalue (Transformation|GetWorldRotation _arrow) "1.000000,1.000000,1.000000") "Undefined" "MultiplyWithRoot" 0 0 0))
  (Game|BindEventtoOnDestroyed _returnvalue_2 (EventDispatchers|CreateEvent :!event Custom|RespawnAfterDeath)))

(event Custom|RespawnAfterDeath
  (params (DestroyedActor :type Actor%20Object%20Reference))
  (Utilities|Time|SetTimerbyEvent (delegate Custom|R) 1.0))

(event Custom|R
  (bind _arrow (Variables|Default|GetArrow))
  (bind _returnvalue (Transformation|GetWorldLocation _arrow))
  (Audio|SpawnSoundatLocation "/Game/Sound/Sounds/MSS_GhostSpawn.MSS_GhostSpawn" _returnvalue "0, 0, 0" 1.0 1.0 0.0 0 "/Game/Sound/Sounds/SC_GhostSpawn.SC_GhostSpawn")
  (Utilities|FlowControl|Delay 0.2)
  (bind _returnvalue_2 (Game|SpawnActorfromClass "/Game/Enemies/AI/BPAI_Skull.BPAI_Skull_C" (Math|Transform|MakeTransform _returnvalue (Transformation|GetWorldRotation _arrow) "1.000000,1.000000,1.000000") "Undefined" "MultiplyWithRoot" 0 0 0))
  (Game|BindEventtoOnDestroyed _returnvalue_2 (EventDispatchers|CreateEvent :!event Custom|RespawnAfterDeath)))

(event EventBeginPlay
  (CallFunction|Respawn))

(fn ConstructionScript)