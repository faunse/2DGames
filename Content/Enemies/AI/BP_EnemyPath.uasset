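; BP_EnemyPath is a patrol path for enemy AI, defined by the EnemyPath spline.
; GetPoints returns the world location of the spline point at the current index.
; IncrementEnemyPath steps that index by Direction and reverses it at the first and last points, giving a back-and-forth route.
; The current index and direction are stored on the path itself.
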(event Custom|IncrementEnemyPath
  (bind _output_get (Variables|Default|SetIndexCurrent (+ (Variables|Default|GetIndexCurrent) (Variables|Default|GetDirection))))
  (if (== _output_get (- (Spline|GetNumberOfSplinePoints (Variables|Default|GetEnemyPath)) 1))
    (Variables|Default|SetDirection -1)
    (elif (== (Variables|Default|GetIndexCurrent) 0)
      (Variables|Default|SetDirection 1))))

(fn ConstructionScript)

(fn GetPoints
  (return (Spline|GetLocationatSplinePoint (Variables|Default|GetEnemyPath) (Variables|Default|GetIndexCurrent) "World")))