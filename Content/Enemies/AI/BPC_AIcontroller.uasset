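; AI controller for ground enemies that starts their behavior tree and sets up its blackboard state.
; On BeginPlay it runs BT_GroundAi and sets the States key to the first E_States entry.
; Both AI Perception update events share a check for the player character, but that branch is empty.
; A debug print and a switch to the second state are left disconnected, so perception never changes the state.
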(event OnPerceptionUpdated(AIPerception)
  (params (UpdatedActors :type Array%20of%20Actor%20Object%20References))
  (if (== (stale OnTargetPerceptionUpdated(AIPerception) Actor) (Game|GetPlayerCharacter 0))
    _))

(event OnTargetPerceptionUpdated(AIPerception)
  (params (Actor :type Actor%20Object%20Reference) (Stimulus :type AI%20Stimulus%20Structure))
  (if (== Actor (Game|GetPlayerCharacter 0))
    _))

(event EventBeginPlay
  (AI|RunBehaviorTree "/Game/Enemies/AI/BT_GroundAi.BT_GroundAi")
  (AI|Components|Blackboard|SetValueasEnum (AI|GetBlackboard 0) (Utilities|Name|MakeLiteralName "States") (Utilities|Enum|LiteralenumE_States "NewEnumerator0")))

(fn ConstructionScript)