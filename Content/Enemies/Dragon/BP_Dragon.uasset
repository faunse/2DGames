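; Dragon boss with a sprite body that runs a repeating fight cycle once BeginFight plays its entrance.
; Timelines move it between set locations while looping timers spawn BP_FireAttack in random-length volleys at three stops.
; It is invincible while attacking, then stops its fire and flashes during a vulnerable window before restarting.
; Damage goes to BPCHealth with a material flash, and Die disables two wall colliders and destroys the actor.
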(event Custom|BeginFight
  ;[1 0 0] Fight Code
  (Variables|Default|SetStartingLocation2 (Transformation|GetActorLocation))
  (bind _enter (Timeline|Entrance PlayFromStart)
    (:Update
      (Transformation|SetActorLocation (Math|Vector|Lerp(Vector) (Variables|Default|GetStartingLocation2) (Math|Vector|MakeVector (- (.x (Variables|Default|GetStartingLocation2)) 2.5e+02) (.y (Variables|Default|GetStartingLocation2)) (.z (Variables|Default|GetStartingLocation2))) _enter) false false))
    (:Finished
      (Class|PaperZDAnimInstance|JumptoNode (Variables|/Script/PaperZD.PaperZDAnimationComponent|GetAnimInstance (Variables|Default|GetAnimationComponent)) "Fire" "None")
      (Utilities|Time|SetTimerbyEvent (delegate Custom|StartFightNow) 1.6))))

(event Custom|Attack3
  (bind _material (Variables|Default|Getmaterial))
  (bind _arrow1 (Variables|Default|GetArrow1))
  ;[1 0 0] Fight Code
  (Class|PaperZDAnimInstance|JumptoNode (Variables|/Script/PaperZD.PaperZDAnimationComponent|GetAnimInstance (Variables|Default|GetAnimationComponent)) "Attack" "None")
  (Utilities|FlowControl|Delay 0.5)
  (Game|SpawnActorfromClass "/Game/Enemies/Dragon/BP_FireAttack.BP_FireAttack_C" (Math|Transform|MakeTransform (Transformation|GetWorldLocation _arrow1) (Transformation|GetWorldRotation _arrow1) "1.000000,1.000000,1.000000") "Undefined" "MultiplyWithRoot" 0 0)
  (Math|Integer|IncrementInt (Variables|Default|GetAttackCount)
    (:%20%20
      (if (>= (Variables|Default|GetAttackCount) (Variables|Default|GetAttackCounter))
        (Utilities|Time|ClearandInvalidateTimerbyHandle (Variables|Default|GetAttack3Timer))
        (Variables|Default|SetAttackCount 0)
        (Variables|Default|SetAttackCounter (Math|Random|RandomIntegerinRange 3 5))
        (Default|StopFire (Variables|Default|GetFire))
        (bind _newtrack_0 (Timeline|Timeline_1 PlayFromStart)
          (:Update
            (Transformation|SetActorLocation (Math|Vector|Lerp(Vector) (Variables|Default|GetLocation3) (Variables|Default|GetLocation4) _newtrack_0) false false))
          (:Finished
            (Variables|Default|SetInvincible false)
            (bind _newtrack_0_2 (Timeline|Flash PlayFromStart)
              (:Update
                (Rendering|Material|SetScalarParameterValue _material "Flash" _newtrack_0_2 :!class /Script/Engine.MaterialInstanceDynamic)
                (Rendering|Material|SetVectorParameterValue _material "FlashColour" "(R=0.921875,G=0.921875,B=0.921875,A=1.000000)" :!class /Script/Engine.MaterialInstanceDynamic))
              (:Finished
                (Utilities|Time|SetTimerbyEvent (delegate Custom|Reset) 5.0)))))))))

(event Custom|Attack1
  (bind _arrow1 (Variables|Default|GetArrow1))
  ;[1 0 0] Fight Code
  (Development|PrintString "1" true true "(R=1.000000,G=0.041194,B=0.000000,A=1.000000)" 1e+01)
  (Class|PaperZDAnimInstance|JumptoNode (Variables|/Script/PaperZD.PaperZDAnimationComponent|GetAnimInstance (Variables|Default|GetAnimationComponent)) "Attack" "None")
  (Utilities|FlowControl|Delay 0.5)
  (Game|SpawnActorfromClass "/Game/Enemies/Dragon/BP_FireAttack.BP_FireAttack_C" (Math|Transform|MakeTransform (Transformation|GetWorldLocation _arrow1) (Transformation|GetWorldRotation _arrow1) "1.000000,1.000000,1.000000") "Undefined" "MultiplyWithRoot" 0 0)
  (Math|Integer|IncrementInt (Variables|Default|GetAttackCount)
    (:%20%20
      (if (>= (Variables|Default|GetAttackCount) (Variables|Default|GetAttackCounter))
        (Utilities|Time|ClearandInvalidateTimerbyHandle (Variables|Default|GetAttack1Timer))
        (Variables|Default|SetAttackCount 0)
        (Variables|Default|SetAttackCounter (Math|Random|RandomIntegerinRange 3 5))
        (bind _newtrack_0 (Timeline|Timeline PlayFromStart)
          (:Update
            (Transformation|SetActorLocation (Math|Vector|Lerp(Vector) (Variables|Default|GetLocation1) (Variables|Default|GetLocation2) _newtrack_0) false false))
          (:Finished
            (bind _returnvalue (Utilities|Time|SetTimerbyEvent (delegate Custom|Attack2) 1.0 true))
            (Variables|Default|SetAttack2timer _returnvalue)))))))

(event Custom|Die
  (bind _wall2 (Variables|Default|GetWall2))
  (bind _wall1 (Variables|Default|GetWall1))
  (bind _box (Variables|/Game/InvisibleWall_BP.InvisibleWall_BP_C|GetBox _wall1))
  (bind _box_2 (Variables|/Game/InvisibleWall_BP.InvisibleWall_BP_C|GetBox _wall2))
  ;[1 1 1] Death
  (Collision|SetCollisionEnabled _box "NoCollision")
  (Collision|SetCollisionResponsetoAllChannels _box "ECR_Ignore")
  (Collision|SetCollisionEnabled _box_2 "NoCollision")
  (Collision|SetCollisionResponsetoAllChannels _box_2 "ECR_Ignore")
  (Actor|DestroyActor))

(event Custom|Attack2
  (bind _arrow1 (Variables|Default|GetArrow1))
  ;[1 0 0] Fight Code
  (Development|PrintString "2" true true "(R=0.000000,G=1.000000,B=0.296419,A=1.000000)" 1e+01)
  (Class|PaperZDAnimInstance|JumptoNode (Variables|/Script/PaperZD.PaperZDAnimationComponent|GetAnimInstance (Variables|Default|GetAnimationComponent)) "Attack" "None")
  (Utilities|FlowControl|Delay 0.5)
  (Game|SpawnActorfromClass "/Game/Enemies/Dragon/BP_FireAttack.BP_FireAttack_C" (Math|Transform|MakeTransform (Transformation|GetWorldLocation _arrow1) (Transformation|GetWorldRotation _arrow1) "1.000000,1.000000,1.000000") "Undefined" "MultiplyWithRoot" 0 0)
  (Math|Integer|IncrementInt (Variables|Default|GetAttackCount)
    (:%20%20
      (if (>= (Variables|Default|GetAttackCount) (Variables|Default|GetAttackCounter))
        (Utilities|Time|ClearandInvalidateTimerbyHandle (Variables|Default|GetAttack2timer))
        (Variables|Default|SetAttackCount 0)
        (Variables|Default|SetAttackCounter (Math|Random|RandomIntegerinRange 3 5))
        (bind _newtrack_0 (Timeline|Timeline_0 PlayFromStart)
          (:Update
            (Transformation|SetActorLocation (Math|Vector|Lerp(Vector) (Variables|Default|GetLocation2) (Variables|Default|GetLocation3) _newtrack_0) false false))
          (:Finished
            (bind _returnvalue (Utilities|Time|SetTimerbyEvent (delegate Custom|Attack3) 1.0 true))
            (Variables|Default|SetAttack3Timer _returnvalue)))))))

(event Custom|StartFightNow
  ;[1 0 0] Fight Code
  (Variables|Default|SetStartingLocation (Transformation|GetActorLocation))
  (Default|StartFire (Variables|Default|GetFire))
  (Variables|Default|SetInvincible true)
  (bind _newtrack_0 (Timeline|MoveTo PlayFromStart)
    (:Update
      (Transformation|SetActorLocation (Math|Vector|Lerp(Vector) (Variables|Default|GetStartingLocation) (Variables|Default|GetLocation1) _newtrack_0) false false))
    (:Finished
      (bind _returnvalue (Utilities|Time|SetTimerbyEvent (delegate Custom|Attack1) 1.0 true))
      (Variables|Default|SetAttack1Timer _returnvalue))))

(event Custom|Stun
  ;[1 0 0] Fight Code
  (Variables|Default|SetStartingLocation (Transformation|GetActorLocation))
  (Default|StartFire (Variables|Default|GetFire))
  (Variables|Default|SetInvincible true)
  (bind _newtrack_0 (Timeline|MoveTo PlayFromStart)
    (:Update
      (Transformation|SetActorLocation (Math|Vector|Lerp(Vector) (Variables|Default|GetStartingLocation) (Variables|Default|GetLocation1) _newtrack_0) false false))
    (:Finished
      (bind _returnvalue (Utilities|Time|SetTimerbyEvent (delegate Custom|Attack1) 1.0 true))
      (Variables|Default|SetAttack1Timer _returnvalue))))

(event Custom|Reset
  ;[1 0 0] Fight Code
  (Class|PaperZDAnimInstance|JumptoNode (Variables|/Script/PaperZD.PaperZDAnimationComponent|GetAnimInstance (Variables|Default|GetAnimationComponent)) "Fire" "None")
  (Utilities|Time|SetTimerbyEvent (delegate Custom|Stun) 1.6))

(event EventBeginPlay
  (Variables|Default|SetAttackCounter (Math|Random|RandomIntegerinRange 3 5))
  (bind _returnvalue (Rendering|Material|CreateDynamicMaterialInstance (Variables|Default|GetSprite) 0 0 "None" :!class /Script/Engine.PrimitiveComponent))
  (Variables|Default|Setmaterial _returnvalue)
  (EventDispatchers|BindEventtoDeath (Variables|Default|GetBPC_Health) (EventDispatchers|CreateEvent :!event Custom|Die)))

(event EventApply/TakeDamage
  (params (Damaged%20Actor :type Actor%20Object%20Reference) (Damage%20amount :type Float%20%28double-precision%29) (Damage%20type :type E_DamageTypes%20Enum :default "NewEnumerator0") (Damage%20Causer :type Actor%20Object%20Reference))
  (bind _self self)
  (bind _material (Variables|Default|GetMaterial))
  (if (not (Variables|Default|GetInvincible))
    (Default|Damaged (Variables|Default|GetBPC_Health) Damaged%20Actor Damage%20amount Damage%20type 0 Damage%20Causer)
    (Utilities|IsValid _self
      (:Is%20Valid
        (bind (_direction _invincibletime _newtrack_1) (Timeline|Timeline_2 PlayFromStart)
          (:Update
            (Utilities|IsValid _self
              (:Is%20Valid
                (Rendering|Material|SetScalarParameterValue _material "Flash" _invincibletime :!class /Script/Engine.MaterialInstanceDynamic)
                (Rendering|Material|SetVectorParameterValue _material "FlashColour" _newtrack_1 :!class /Script/Engine.MaterialInstanceDynamic))
              (:Is%20Not%20Valid
                (Timeline|Timeline_2 Stop)))))))))

(fn ConstructionScript)