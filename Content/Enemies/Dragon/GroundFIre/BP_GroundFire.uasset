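; Ground fire hazard for the dragon enemy, built from paper flipbooks that damage the player standing in them while lit.
; It starts hidden and inactive, with StartFire and StopFire toggling the Stopped flag and the visibility of all flipbooks.
; Box overlap applies damage immediately and starts a looping Check timer that repeats it using the last overlapping actor.
; Check clears the timer once the player is no longer in the PlayerCheck array.
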(event OnComponentBeginOverlap(Box)
  (params (OverlappedComponent :type Primitive%20Component%20Object%20Reference) (OtherActor :type Actor%20Object%20Reference) (OtherComp :type Primitive%20Component%20Object%20Reference) (OtherBodyIndex :type Integer) (bFromSweep :type Boolean) (SweepResult :type Hit%20Result%20Structure%20%28by%20ref%29))
  (Utilities|Array|Add (Variables|Default|GetPlayerCheck) OtherActor)
  (Utilities|FlowControl|Sequence
    (:then_0
      (bind _returnvalue (Utilities|Time|SetTimerbyEvent (delegate Custom|Check) 0.2 true))
      (bind _output_get (Variables|Default|SetCheckTimer _returnvalue)))
    (:then_1
      (if (and (== OtherActor (Game|GetPlayerCharacter 0)) (== (Variables|Default|GetStopped) false))
        (Class|BPIDamage|Apply/TakeDamage(Message) OtherActor OtherActor 1.0 "NewEnumerator0")))))

(event OnComponentEndOverlap(Box)
  (params (OverlappedComponent :type Primitive%20Component%20Object%20Reference) (OtherActor :type Actor%20Object%20Reference) (OtherComp :type Primitive%20Component%20Object%20Reference) (OtherBodyIndex :type Integer))
  (if (== OtherActor (Game|GetPlayerCharacter 0))
    (Utilities|Array|Clear (Variables|Default|GetPlayerCheck))))

(event Custom|StopFire
  ;[1 1 1] Starts and stops fire
  (Variables|Default|SetStopped true)
  (Rendering|SetVisibility (Variables|Default|GetFlipBookArray) false false))

(event Custom|StartFire
  ;[1 1 1] Starts and stops fire
  (Variables|Default|SetStopped false)
  (Rendering|SetVisibility (Variables|Default|GetFlipBookArray) true false))

(event Custom|Check
  (bind _returnvalue (Game|GetPlayerCharacter 0))
  (if (== (Utilities|Array|FindItem (Variables|Default|GetPlayerCheck) _returnvalue) -1)
    (Utilities|Time|ClearandInvalidateTimerbyHandle (stale OnComponentBeginOverlap(Box) _output_get))
    (elif (and (== (stale OnComponentBeginOverlap(Box) OtherActor) _returnvalue) (== (Variables|Default|GetStopped) false))
      (Class|BPIDamage|Apply/TakeDamage(Message) (stale OnComponentBeginOverlap(Box) OtherActor) (stale OnComponentBeginOverlap(Box) OtherActor) 1.0 "NewEnumerator0"))))

(event EventBeginPlay
  ;[1 1 1] Makes array of flipbooks to make life easier
  (Variables|Default|SetStopped true)
  (bind _output_get (Variables|Default|SetFlipBookArray (Utilities|Array|MakeArray (Variables|Default|GetPaperFlipbook13) (Variables|Default|GetPaperFlipbook5) (Variables|Default|GetPaperFlipbook6) (Variables|Default|GetPaperFlipbook7) (Variables|Default|GetPaperFlipbook8) (Variables|Default|GetPaperFlipbook) (Variables|Default|GetPaperFlipbook1) (Variables|Default|GetPaperFlipbook4) (Variables|Default|GetPaperFlipbook2) (Variables|Default|GetPaperFlipbook3) (Variables|Default|GetPaperFlipbook9) (Variables|Default|GetPaperFlipbook16) (Variables|Default|GetPaperFlipbook17) (Variables|Default|GetPaperFlipbook15) (Variables|Default|GetPaperFlipbook11) (Variables|Default|GetPaperFlipbook12) (Variables|Default|GetPaperFlipbook10) (Variables|Default|GetPaperFlipbook14))))
  (Rendering|SetVisibility _output_get false false))

(fn ConstructionScript)