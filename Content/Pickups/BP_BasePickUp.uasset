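; Base pickup actor that the player character collects once by overlapping its box.
; The construction script fills its pickup struct from the DT_PickUps row named after its pickup type.
; On overlap it sends amount and type to the player via PickupMessage, switches its flipbook to a pop, plays a sound with concurrency settings, and destroys itself after a short timer.
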(event OnComponentBeginOverlap(Box)
  (params (OverlappedComponent :type Primitive%20Component%20Object%20Reference) (OtherActor :type Actor%20Object%20Reference) (OtherComp :type Primitive%20Component%20Object%20Reference) (OtherBodyIndex :type Integer) (bFromSweep :type Boolean) (SweepResult :type Hit%20Result%20Structure%20%28by%20ref%29))
  (bind _s_pickup (Variables|Default|GetS_Pickup))
  (if (== OtherActor (Game|GetPlayerCharacter 0))
    (Utilities|FlowControl|DoOnce false
      (:Completed
        (Class|BPIPickUp|Pickup(Message) OtherActor (.amount _s_pickup) (.pickup _s_pickup))
        (CallFunction|FX)
        (Utilities|Time|SetTimerbyEvent (delegate Custom|Explode) 0.5)))))

(event Custom|FX
  (Sprite|SetFlipbook (Variables|Default|GetPaperFlipbook) "/Game/Art/Gem/Gems/FB_Pop.FB_Pop")
  (Audio|PlaySoundatLocation "/Game/Sound/Sounds/MSS_Pickup.MSS_Pickup" (Transformation|GetActorLocation) "0, 0, 0" 1.0 1.0 0.0 0 "/Game/Sound/Sounds/SC_PickUp.SC_PickUp" 0 0))

(event Custom|Explode
  (Actor|DestroyActor))

(fn ConstructionScript
  (bind _returnvalue (Utilities|GetDataTableRow "/Game/Pickups/DT_PickUps.DT_PickUps" (Utilities|String|StringToName (Utilities|String|EnumtoString (.Pickup (Utilities|Struct|BreakS_PickUps (Variables|Default|GetS_Pickup))))))
    (:then
      (Variables|Default|SetS_Pickup _returnvalue))))