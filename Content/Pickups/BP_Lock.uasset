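; BP_Lock is a Paper2D lock that acts as a gated exit to another level.
; OpenDoor sets the Open flag, switches to the unlocked flipbook, then destroys that flipbook component after a short timer.
; The box remains as the trigger, loading LevelName when the player character begins overlapping it while Open is true.
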(event OnComponentBeginOverlap(Box)
  (params (OverlappedComponent :type Primitive%20Component%20Object%20Reference) (OtherActor :type Actor%20Object%20Reference) (OtherComp :type Primitive%20Component%20Object%20Reference) (OtherBodyIndex :type Integer) (bFromSweep :type Boolean) (SweepResult :type Hit%20Result%20Structure%20%28by%20ref%29))
  (if (== OtherActor (Game|GetPlayerCharacter 0))
    (if (Variables|Default|GetOpen)
      (Game|OpenLevel(byName) (Variables|Default|GetLevelName)))))

(event Custom|OpenDoor
  (Variables|Default|SetOpen true)
  (Sprite|SetFlipbook (Variables|Default|GetPaperFlipbook) "/Game/Art/Lock/FB_LockOpen.FB_LockOpen")
  (Utilities|Time|SetTimerbyEvent (delegate Custom|D) 0.3))

(event Custom|D
  (Components|DestroyComponent (Variables|Default|GetPaperFlipbook)))

(fn ConstructionScript)